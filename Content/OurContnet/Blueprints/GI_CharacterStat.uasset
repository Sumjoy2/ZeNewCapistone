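; GI_CharacterStat holds combat stats for the selected character class, likely as a Game Instance judging by its name.
; Its ClassSelect event switches on Selector across Normal, Tank, Melee, Flammer and Healer.
; Each branch writes hardcoded damage, speed, health and fire rate into shared variables, with health the same for every class.
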(event `ClassSelect`
  (switch `/Game/OurContnet/Blueprints/E_ClassSelect` (`self.Selector`)
    (:`NewEnumerator0`
      (set `self.DMG` 10.0)
      (set `self.SPD` 750.0)
      (set `self.HP` 100.0)
      (set `self.fireRate` 0.095))
    (:`NewEnumerator1`
      (set `self.DMG` 20.0)
      (set `self.SPD` 600.0)
      (set `self.HP` 100.0)
      (set `self.fireRate` 1.5))
    (:`NewEnumerator2`
      (set `self.DMG` 20.0)
      (set `self.SPD` 900.0)
      (set `self.HP` 100.0)
      (set `self.fireRate` 0.2))
    (:`NewEnumerator3`
      (set `self.DMG` 4.0)
      (set `self.SPD` 750.0)
      (set `self.HP` 100.0)
      (set `self.fireRate` 0.05))
    (:`NewEnumerator4`
      (set `self.DMG` 20.0)
      (set `self.SPD` 800.0)
      (set `self.HP` 100.0)
      (set `self.fireRate` 1.0))))