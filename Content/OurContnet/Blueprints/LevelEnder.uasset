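; LevelEnder is a trigger actor that advances the game to the next level when the first-person character overlaps its box.
; It caches the GI_CharacterStat game instance on BeginPlay and reads the current index and level-name list from it.
; On overlap it opens the next listed level by name and updates the stored index, wrapping to the first level after the last.
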(event `self.ReceiveBeginPlay`
  (bind _asgi_character_stat (cast `/Game/OurContnet/Blueprints/GI_CharacterStat` (`GameplayStatics.GetGameInstance`)))
  (set `self.As GI Character Stat` _asgi_character_stat))

(event `self.Box.OnComponentBeginOverlap`
  (params (OverlappedComponent :type "PrimitiveComponent Object Reference") (OtherActor :type "Actor Object Reference") (OtherComp :type "PrimitiveComponent Object Reference") (OtherBodyIndex :type Integer) (bFromSweep :type Boolean) (SweepResult :type "HitResult Structure (by ref)"))
  (bind _levelholder (`/Game/OurContnet/Blueprints/GI_CharacterStat.LevelHolder` (`self.As GI Character Stat`)))
  (bind _returnvalue (+ (`/Game/OurContnet/Blueprints/GI_CharacterStat.CurrentLevel` (`self.As GI Character Stat`)) 1))
  (cast `/Game/FirstPerson/Blueprints/BP_FirstPersonCharacter` OtherActor)
  (if (> _returnvalue (- (`KismetArrayLibrary.Array_Length` _levelholder) 1))
    (set `/Game/OurContnet/Blueprints/GI_CharacterStat.CurrentLevel` 0 (`self.As GI Character Stat`))
    (`GameplayStatics.OpenLevel` (`|GetArrayItem` (`/Game/OurContnet/Blueprints/GI_CharacterStat.LevelHolder` (`self.As GI Character Stat`))))
    (else
      (`GameplayStatics.OpenLevel` (`|GetArrayItem` _levelholder _returnvalue))
      (set `/Game/OurContnet/Blueprints/GI_CharacterStat.CurrentLevel` _returnvalue (`self.As GI Character Stat`)))))

(fn `UserConstructionScript`)