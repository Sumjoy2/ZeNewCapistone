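; Dummy is a target enemy with a health bar widget that respawns itself when killed.
; Any hit on its Box component subtracts a fixed amount of clamped health and updates the Helth widget.
; At zero health it spawns a fresh Dummy, slightly offset along X, and destroys itself.
; Each tick, after a one-frame delay, the widget yaws to face the player camera.
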(event `self.ReceiveBeginPlay`
  (bind _output_get (set `self.MaxHealth` 100.0))
  (set `self.Health` _output_get)
  (bind _ashelth (cast `/Game/OurContnet/Widgets/Helth` (`WidgetComponent.GetUserWidgetObject` (`self.Widget`))))
  (bind _output_get_2 (set `self.As Helth` _ashelth))
  (set `/Game/OurContnet/Widgets/Helth.HelthMax` (`self.MaxHealth`) _output_get_2)
  (bind _output_get_3 (set `/Game/OurContnet/Widgets/Helth.Curhelth` (`self.Health`) _output_get_2))
  (`/Game/OurContnet/Widgets/Helth.HelthUpdate` _output_get_2 _output_get_3))

(event `self.ReceiveTick`
  (params (DeltaSeconds :type "Float (single-precision)"))
  (`KismetSystemLibrary.DelayUntilNextTick`)
  (`self.FollowCamera`))

(event `self.Box.OnComponentHit`
  (params (HitComponent :type "PrimitiveComponent Object Reference") (OtherActor :type "Actor Object Reference") (OtherComp :type "PrimitiveComponent Object Reference") (NormalImpulse :type "Vector Structure") (Hit :type "HitResult Structure (by ref)"))
  (`self.ModifyHealth` 25.0))

(fn `FollowCamera`
  (bind (_returnvalue_roll _returnvalue_pitch _returnvalue_yaw) (`KismetMathLibrary.BreakRotator` (`KismetMathLibrary.FindLookAtRotation` (`SceneComponent.K2_GetComponentLocation` (`self.Widget`)) (`PlayerCameraManager.GetCameraLocation` (`GameplayStatics.GetPlayerCameraManager` 0)))))
  (`SceneComponent.K2_SetWorldRotation` (`self.Widget`) (`KismetMathLibrary.MakeRotator` 0.0 0.0 _returnvalue_yaw) false false))

(fn `ModifyHealth`
  (params (HealthSubtrazt :type "Float (double-precision)"))
  (bind (_returnvalue_location _returnvalue_rotation _returnvalue_scale) (`KismetMathLibrary.BreakTransform` (`self.GetTransform`)))
  (bind _output_get (set `self.Health` (`KismetMathLibrary.FClamp` (- (`self.Health`) HealthSubtrazt) 0.0 (`self.MaxHealth`))))
  (`/Game/OurContnet/Widgets/Helth.HelthUpdate` (`self.As Helth`) _output_get)
  (if (<= (`self.Health`) 0.0)
    (`|SpawnActorFromClass` "Dummy_C" (`KismetMathLibrary.MakeTransform` (+ _returnvalue_location (-10.0 0.0 0.0)) _returnvalue_rotation _returnvalue_scale) "Undefined" "MultiplyWithRoot" null null)
    (`self.K2_DestroyActor`)))

(fn `UserConstructionScript`)